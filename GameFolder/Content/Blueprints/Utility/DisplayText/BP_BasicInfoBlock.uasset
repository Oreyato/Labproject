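; BP_BasicInfoBlock is a display-text utility actor that shows a configurable label with a block and a separator.
; Its construction script applies the input text and color to both Text and ReversedText, and sets the block and separator materials.
; It then sizes the separator to the label, deriving its world X scale from the text's local Y size plus a small margin.
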(fn ConstructionScript
  (bind _inputtext (Variables|Default|GetInputText))
  (bind _textcolor (Variables|Default|GetTextColor))
  (bind _separator (Variables|Default|GetSeparator))
  (bind _returnvalue (Utilities|Text|ToText(String) _inputtext))
  (bind _returnvalue_2 (Transformation|GetWorldTransform _separator))
  ;[1 1 1] Text Relative Code
  (Rendering|Components|TextRender|SetText (Variables|Default|GetText) _returnvalue)
  (Rendering|Components|TextRender|SetText (Variables|Default|GetReversedText) _returnvalue)
  (Rendering|Components|TextRender|SetTextRenderColor (Variables|Default|GetText) _textcolor)
  (Rendering|Components|TextRender|SetTextRenderColor (Variables|Default|GetReversedText) _textcolor)
  ;[1 1 1] Materials
  (Rendering|Material|SetMaterial (Variables|Default|GetBlock) 0 (Variables|Default|GetBlockMaterial))
  (Rendering|Material|SetMaterial (Variables|Default|GetSeparator) 0 (Variables|Default|GetSeparatorMaterial))
  ;[1 1 1] Adapt separator size to text size
  (Transformation|SetWorldTransform _separator (Math|Transform|MakeTransform (.location _returnvalue_2) (.rotation _returnvalue_2) (Math|Vector|MakeVector (+ (/ (.y (Class|TextRenderComponent|GetTextLocalSize (Variables|Default|GetText))) 1e+02) 0.1) (.y (.scale _returnvalue_2)) (.z (.scale _returnvalue_2)))) false false))