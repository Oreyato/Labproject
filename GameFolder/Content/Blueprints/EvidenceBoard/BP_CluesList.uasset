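; BP_CluesList holds the list of clues for the evidence board, loaded from the DT_Clues data table.
; The Construction Script looks up rows named by index, from zero up to CluesNumber, and appends each one found to the Clues array.
; On BeginPlay it prints a selection message naming the clue at the ClueTest index, which appears to be a test readout.
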(event EventBeginPlay
  (Development|PrintString (Utilities|String|Append "Select " (.name (Utilities|Struct|BreakStruct_Clue (Utilities|Array|Get(acopy) (Variables|Default|Getclues) (Variables|Default|GetclueTest)))) " clue")))

(fn ConstructionScript
  (for _index (range 0 (- (Variables|Default|GetcluesNumber) 1))
    (bind _returnvalue (Utilities|GetDataTableRow "/Game/Blueprints/EvidenceBoard/DT_Clues.DT_Clues" (Utilities|String|StringToName (Utilities|String|ToString(Integer) _index)))
      (:then
        (Utilities|Array|Add (Variables|Default|Getclues) _returnvalue)))))