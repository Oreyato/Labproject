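; Clickable image plane actor in the EvidenceBoard folder that opens the level set in ChoiceLevel when clicked.
; On BeginPlay it applies its material instance and enables mouse-over events on the player controller.
; Hovering switches the cursor to a grab hand and leaving restores the default.
; The construction script sizes the plane from Scale and the texture's width-to-height ratio so the image keeps its proportions.
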(event OnClicked(Plane)
  (params (TouchedComponent :type Primitive%20Component%20Object%20Reference) (ButtonPressed :type Key%20Structure :default "None"))
  (Game|OpenLevel(byObjectReference) (Variables|Default|GetChoiceLevel)))

(event OnBeginCursorOver(Plane)
  (params (TouchedComponent :type Primitive%20Component%20Object%20Reference))
  (Variables|/Script/Engine.PlayerController|SetCurrentMouseCursor (Game|GetPlayerController 0) "GrabHand"))

(event OnEndCursorOver(Plane)
  (params (TouchedComponent :type Primitive%20Component%20Object%20Reference))
  (Variables|/Script/Engine.PlayerController|SetCurrentMouseCursor (Game|GetPlayerController 0) "Default"))

(event EventBeginPlay
  (Rendering|Material|SetMaterial (Variables|Default|GetPlane) 0 (Variables|Default|GetMaterial%20Instance))
  (Variables|/Script/Engine.PlayerController|SetbEnableMouseOverEvents (Game|GetPlayerController 0) true))

(event Collision|EventActorBeginOverlap
  (params (OtherActor :type Actor%20Object%20Reference)))

(event EventTick
  (params (DeltaSeconds :type Float%20%28single-precision%29)))

(fn ConstructionScript
  (bind _scale (Variables|Default|GetScale))
  (bind _texture (Variables|Default|GetTexture))
  (Transformation|SetWorldScale3D (Variables|Default|GetPlane) (Math|Vector|MakeVector (* _scale (/ (Math|Conversions|ToFloat(Integer) (Class|Texture2D|BlueprintGetSizeX _texture)) (Math|Conversions|ToFloat(Integer) (Class|Texture2D|BlueprintGetSizeY _texture)))) _scale 1.0)))