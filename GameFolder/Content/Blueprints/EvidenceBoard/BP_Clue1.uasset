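; BP_Clue1 is an evidence board clue Blueprint that holds the data describing a clue.
; On BeginPlay it copies the fields of its StructClue into separate variables for name, position displacement, texture, unlock state, category and scale.
; It then looks up DT_Clues rows by numeric row name over a fixed index range and prints each found clue's name, without storing the row data.
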(event EventBeginPlay
  (bind _struct_clue (Variables|ClueSpecs|GetStruct%20Clue))
  (bind (_name _positiondisplacement _texture _zone _isunlocked _category _scale) (Utilities|Struct|BreakStruct_Clue _struct_clue))
  (Variables|ClueSpecs|SetName _name)
  (Variables|ClueSpecs|SetPosition%20Displacement _positiondisplacement)
  (Variables|ClueSpecs|SetTexture _texture)
  (Variables|ClueSpecs|SetIs%20Unlocked _isunlocked)
  (Variables|ClueSpecs|SetCategory _category)
  (Variables|ClueSpecs|SetScale _scale)
  (for _index (range 0 25)
    (bind _returnvalue (Utilities|GetDataTableRow "/Game/Blueprints/EvidenceBoard/DT_Clues.DT_Clues" (Utilities|String|StringToName (Utilities|String|ToString(Integer) _index)))
      (:then
        (Development|PrintString (.name (Utilities|Struct|BreakStruct_Clue _returnvalue)))))))

(fn ConstructionScript)