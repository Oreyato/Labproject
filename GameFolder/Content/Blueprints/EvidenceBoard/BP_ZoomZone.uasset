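; Clickable zone on the evidence board that displays its clues and lets the player zoom the evidence camera onto it.
; Hovering shifts the zone along X; clicking zooms in, and clicking again or leaving zooms out, with timelines gating input.
; On BeginPlay it spawns meshes for its DT_Clues rows, using dynamic materials that show grey for locked clues.
; Clue scale is divided by the zone's construction-time scale to offset it.
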(event OnBeginCursorOver(Plane)
  (params (TouchedComponent :type Primitive%20Component%20Object%20Reference))
  (bind _defaultsceneroot (Variables|Default|GetDefaultSceneRoot))
  (bind _returnvalue (Transformation|GetWorldTransform _defaultsceneroot))
  (if (not (Variables|Default|GetisZoomedIn))
    (Transformation|SetWorldTransform _defaultsceneroot (Math|Transform|MakeTransform (Math|Vector|MakeVector (+ (* (Variables|Default|GetoveringDisplacement) -1.0) (.x (.location _returnvalue))) (.y (.location _returnvalue)) (.z (.location _returnvalue))) (.rotation _returnvalue) (.scale _returnvalue)) false false)
    (Development|PrintString "Enter")))

(event OnEndCursorOver(Plane)
  (params (TouchedComponent :type Primitive%20Component%20Object%20Reference))
  (if (Variables|Default|GetisZoomedIn)
    (if (Variables|Default|GetcanUpdate)
      (Default|DefaultPos (Variables|Default|GetEvidenceCamera))
      (Variables|Default|SetcanUpdate false)
      (Timeline|Timeline_1 PlayFromStart
        (:Finished
          (Variables|Default|SetcanUpdate true)
          (Variables|Default|SetisZoomedIn false))))
    (else
      (CallFunction|ZoomZonetoInitPos))))

(event OnClicked(Plane)
  (params (TouchedComponent :type Primitive%20Component%20Object%20Reference) (ButtonPressed :type Key%20Structure :default "None"))
  (if (Variables|Default|GetisZoomedIn)
    (if (Variables|Default|GetcanUpdate)
      (Default|DefaultPos (Variables|Default|GetEvidenceCamera))
      (Variables|Default|SetcanUpdate false)
      (Timeline|Timeline_1 PlayFromStart
        (:Finished
          (Variables|Default|SetcanUpdate true)
          (Variables|Default|SetisZoomedIn false))))
    (elif (Variables|Default|GetcanUpdate)
      (CallFunction|ZoomZonetoInitPos)
      (Default|Zoomin (Variables|Default|GetEvidenceCamera) (.location (Transformation|GetWorldTransform (Variables|Default|GetDefaultSceneRoot))))
      (Variables|Default|SetcanUpdate false)
      (Variables|Default|SetisZoomedIn true)
      (Timeline|Timeline_0 PlayFromStart
        (:Finished
          (Variables|Default|SetcanUpdate true))))))

(event EventBeginPlay
  (CallFunction|EnableMouseParameters)
  (Variables|Default|SetinitPos (.location (Transformation|GetWorldTransform (Variables|Default|GetDefaultSceneRoot))))
  (CallFunction|InitClues))

(fn ConstructionScript
  (bind _defaultsceneroot (Variables|Default|GetDefaultSceneRoot))
  (bind _returnvalue (Transformation|GetWorldTransform _defaultsceneroot))
  (Transformation|SetWorldTransform _defaultsceneroot (Math|Transform|MakeTransform (.location _returnvalue) (.rotation _returnvalue) (Variables|Default|GetscaleModif)) false false))

(fn ZoomZonetoInitPos
  (bind _defaultsceneroot (Variables|Default|GetDefaultSceneRoot))
  (bind _returnvalue (Transformation|GetWorldTransform _defaultsceneroot))
  (Transformation|SetWorldTransform _defaultsceneroot (Math|Transform|MakeTransform (Variables|Default|GetinitPos) (.rotation _returnvalue) (.scale _returnvalue)) false false))

(fn EnableMouseParameters
  (bind _returnvalue (Game|GetPlayerController 0))
  (Variables|/Script/Engine.PlayerController|SetbEnableClickEvents _returnvalue true)
  (Variables|/Script/Engine.PlayerController|SetbEnableMouseOverEvents _returnvalue true)
  (Variables|/Script/Engine.PlayerController|SetbShowMouseCursor _returnvalue true)
  (Input|EnableInput _returnvalue))

(fn InitClues
  (for _index (range 0 (- (Variables|Clue|GetcluesNumber) 1))
    (bind _returnvalue (Utilities|GetDataTableRow "/Game/Blueprints/EvidenceBoard/DT_Clues.DT_Clues" (Utilities|String|StringToName (Utilities|String|ToString(Integer) _index)))
      (:then
        (if (Utilities|Enum|Equal(Enum) (Variables|Default|Getzone) (.zone (Utilities|Struct|BreakStruct_Clue _returnvalue)))
          (Utilities|FlowControl|Sequence
            (:then_0
              (bind _rectifiedcluescale (CallFunction|RectifyScale (.texture (Utilities|Struct|BreakStruct_Clue _returnvalue)) (.uniformScale (Utilities|Struct|BreakStruct_Clue _returnvalue))))
              (bind _returnvalue_2 (AddComponent|AddStaticMeshComponent false (Math|Transform|MakeTransform (Math|Vector|MakeVector 0.01 (.y (.positionDisplacement (Utilities|Struct|BreakStruct_Clue _returnvalue))) (.z (.positionDisplacement (Utilities|Struct|BreakStruct_Clue _returnvalue)))) "0.000000,90.000000,90.000000" _rectifiedcluescale)))
              (bind _returnvalue_3 (Rendering|Material|CreateDynamicMaterialInstance _returnvalue_2 0 "/Game/Materials/EvidenceBoard/M_Clue.M_Clue" "None" :!class /Script/Engine.PrimitiveComponent))
              (if (.isUnlocked (Utilities|Struct|BreakStruct_Clue _returnvalue))
                (Rendering|Material|SetTextureParameterValue _returnvalue_3 "Texture" (.texture (Utilities|Struct|BreakStruct_Clue _returnvalue)))
                (else
                  (Rendering|Material|SetTextureParameterValue _returnvalue_3 "Texture" "/Engine/ArtTools/RenderToTexture/Textures/127grey.127grey"))))
            (:then_1
              (Development|PrintString (Utilities|String|Append "Add " (.name (Utilities|Struct|BreakStruct_Clue _returnvalue))) true true "(R=0.000000,G=0.660000,B=1.000000,A=1.000000)" 5.0))))))))

(fn RectifyScale
  (params (texture :type Texture%202D%20Object%20Reference) (uniformScale :type Float%20%28single-precision%29))
  (bind _scalemodif (Variables|Default|GetscaleModif))
  (Utilities|IsValid texture
    (:Is%20Valid
      (return (Math|Vector|MakeVector (/ uniformScale (.x _scalemodif)) (/ uniformScale (.y _scalemodif)) (/ uniformScale (.z _scalemodif)))))
    (:Is%20Not%20Valid
      (return "1.000000,1.000000,1.000000"))))