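; BP_ZoomZone is a hoverable zone actor, filed under the evidence board camera, that shifts when the mouse cursor passes over it.
; On BeginPlay it enables click events, mouse-over events and the cursor on the first player controller.
; Its Plane's cursor-over events offset the root along world X by OveringDisplacement, negatively on enter and back on exit, printing debug text.
; No click or zoom logic is implemented here.
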(event OnBeginCursorOver(Plane)
  (params (TouchedComponent :type Primitive%20Component%20Object%20Reference))
  (bind _defaultsceneroot (Variables|Default|GetDefaultSceneRoot))
  (Class|SceneComponent|AddWorldTransform _defaultsceneroot (Math|Transform|MakeTransform (Math|Vector|MakeVector (* (Variables|Default|GetoveringDisplacement) -1.0) 0.0 0.0) "0, 0, 0" (Transformation|GetWorldScale _defaultsceneroot)) false false)
  (Development|PrintString "Enter"))

(event OnEndCursorOver(Plane)
  (params (TouchedComponent :type Primitive%20Component%20Object%20Reference))
  (bind _defaultsceneroot (Variables|Default|GetDefaultSceneRoot))
  (Class|SceneComponent|AddWorldTransform _defaultsceneroot (Math|Transform|MakeTransform (Math|Vector|MakeVector (Variables|Default|GetoveringDisplacement) 0.0 0.0) "0, 0, 0" (Transformation|GetWorldScale _defaultsceneroot)) false false)
  (Development|PrintString "Exit"))

(event EventBeginPlay
  (bind _returnvalue (Game|GetPlayerController 0))
  (Variables|/Script/Engine.PlayerController|SetbEnableClickEvents _returnvalue true)
  (Variables|/Script/Engine.PlayerController|SetbEnableMouseOverEvents _returnvalue true)
  (Variables|/Script/Engine.PlayerController|SetbShowMouseCursor _returnvalue true))

(event Collision|EventActorBeginOverlap
  (params (OtherActor :type Actor%20Object%20Reference)))

(event EventTick
  (params (DeltaSeconds :type Float%20%28single-precision%29)))

(fn ConstructionScript)