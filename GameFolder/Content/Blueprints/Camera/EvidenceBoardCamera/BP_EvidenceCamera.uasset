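; Evidence board camera pawn that the first player controller possesses on BeginPlay, storing its start location.
; ZoomIn runs a timeline that moves the root to the target's Y and Z while offsetting X by ZoomLevel from where the move began.
; DefaultPos uses a second timeline to return it to the stored start.
; Both lerp from the current location on each update, so the easing compounds beyond the curve.
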(event Custom|ZoomIn
  (params (targetPos :type Vector))
  (bind _defaultsceneroot (Variables|Default|GetDefaultSceneRoot))
  (bind _returnvalue (Transformation|GetWorldLocation _defaultsceneroot))
  (Variables|Default|SetinitPos (Transformation|GetWorldLocation (Variables|Default|GetDefaultSceneRoot)))
  (bind _zoomincurve (Timeline|TL_ZoomIn PlayFromStart)
    (:Update
      (Transformation|SetWorldLocation (Variables|Default|GetDefaultSceneRoot) (Math|Vector|MakeVector (Math|Float|Lerp (.x _returnvalue) (+ (.x (Variables|Default|GetinitPos)) (Variables|Default|GetzoomLevel)) _zoomincurve) (Math|Float|Lerp (.y _returnvalue) (.y targetPos) _zoomincurve) (Math|Float|Lerp (.z _returnvalue) (.z targetPos) _zoomincurve)) false false))))

(event Custom|DefaultPos
  (bind _defaultsceneroot (Variables|Default|GetDefaultSceneRoot))
  (bind _startpos (Variables|Default|GetstartPos))
  (bind _returnvalue (Transformation|GetWorldLocation _defaultsceneroot))
  (bind _zoomincurve (Timeline|Timeline_0 PlayFromStart)
    (:Update
      (Transformation|SetWorldLocation (Variables|Default|GetDefaultSceneRoot) (Math|Vector|MakeVector (Math|Float|Lerp (.x _returnvalue) (.x _startpos) _zoomincurve) (Math|Float|Lerp (.y _returnvalue) (.y _startpos) _zoomincurve) (Math|Float|Lerp (.z _returnvalue) (.z _startpos) _zoomincurve)) false false))))

(event EventBeginPlay
  (Pawn|Possess (Game|GetPlayerController 0) self)
  (Variables|Default|SetstartPos (Transformation|GetWorldLocation (Variables|Default|GetDefaultSceneRoot))))

(event Collision|EventActorBeginOverlap
  (params (OtherActor :type Actor%20Object%20Reference)))

(event EventTick
  (params (DeltaSeconds :type Float%20%28single-precision%29)))

(fn ConstructionScript)