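; BP_Room is a level-camera actor that defines a rectangular room area in the X-Z plane, shown by a plane.
; Its Construction Script places ToSphere at the Displacement offset, then centers and scales Plane to span from FromSphere to ToSphere.
; An Invert flag flips which way the upright plane faces.
; It has no runtime logic, as all event nodes are disabled stubs.
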(event EventBeginPlay)

(event Collision|EventActorBeginOverlap
  (params (OtherActor :type Actor%20Object%20Reference)))

(event EventTick
  (params (DeltaSeconds :type Float%20%28single-precision%29)))

(fn ConstructionScript
  (bind _displacement (Variables|Default|Getdisplacement))
  (Variables|Default|SetfromPos (Transformation|GetWorldLocation (Variables|Default|GetfromSphere)))
  (Transformation|SetRelativeLocation (Variables|Default|GettoSphere) (Math|Vector|MakeVector (.x _displacement) 0.0 (.z _displacement)) false false)
  (Variables|Default|SettoPos (Transformation|GetWorldLocation (Variables|Default|GettoSphere)))
  (Transformation|SetRelativeLocation (Variables|Default|Getplane) (/ (- (Variables|Default|GettoPos) (Variables|Default|GetfromPos)) 2.0) false false)
  (if (Variables|Default|Getinvert)
    (Transformation|SetWorldRotation (Variables|Default|Getplane) (Math|Rotator|MakeRotator -9e+01 0.0 0.0) false false)
    (else
      (Transformation|SetWorldRotation (Variables|Default|Getplane) (Math|Rotator|MakeRotator 9e+01 0.0 0.0) false false)))
  (Transformation|SetWorldScale3D (Variables|Default|Getplane) (Math|Vector|MakeVector (/ (- (.x (Variables|Default|GettoPos)) (.x (Variables|Default|GetfromPos))) 1e+02) (/ (- (.z (Variables|Default|GettoPos)) (.z (Variables|Default|GetfromPos))) 1e+02) 1.0)))