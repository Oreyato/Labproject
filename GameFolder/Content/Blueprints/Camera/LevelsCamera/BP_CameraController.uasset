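; Side-scrolling camera controller that becomes the view target and follows BP_Character through rooms.
; Each tick outside transitions, it clamps camera X to the current room's limits and moves Z only when the player leaves a vertical dead-zone box.
; ChangingRoom pauses following while timelines slide X to the new room's edge, and StairsHeight eases Z to the player's height.
; The construction script applies camera distance and pitch and selects the first room.
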(event Custom|StairsHeight
  (bind _camera (Variables|Default|GetCamera))
  (bind _returnvalue (Transformation|GetWorldLocation _camera))
  ;[1 1 1] Camera z pos after stairs
  (bind _curve (Timeline|Timeline_0 PlayFromStart)
    (:Update
      (Transformation|SetWorldLocation _camera (Math|Vector|MakeVector (.x _returnvalue) (.y _returnvalue) (Math|Float|Lerp (.z _returnvalue) (+ (.z (Transformation|GetWorldLocation (Variables|/Script/Engine.Character|GetCapsuleComponent (Variables|Default|Getplayer)))) (Variables|camera|GetcamVerticalOffset)) _curve)) false false))))

(event Custom|Changing%20Room
  (params (targetRoom :type BP%20Room%20Object%20Reference) (allowTransitions :type Boolean))
  (bind _camera (Variables|Default|GetCamera))
  (bind _camera_2 (Variables|Default|GetCamera))
  (bind _roomlimits (Variables|Room|GetroomLimits))
  (bind _camera_3 (Variables|Default|GetCamera))
  (bind _returnvalue (Transformation|GetWorldLocation _camera_2))
  (bind _returnvalue_2 (Transformation|GetWorldLocation _camera_3))
  ;[1 1 1] Changing Room
  (Utilities|FlowControl|Sequence
    (:then_0
      (bind _output_get (Variables|Room|SetpreviousRoom (Variables|Room|GetcurrentRoom)))
      (bind _output_get_2 (Variables|Room|SetcurrentRoom targetRoom))
      (if (and (!= _output_get_2 (Variables|Room|GetpreviousRoom)) allowTransitions)
        (Variables|Room|SetroomTransition true)
        (Utilities|FlowControl|Sequence
          (:then_0
            (Variables|camera|SetinitXPos (.x _returnvalue))
            ;;[1 1 1] Is coming from left test
            (if (>= (.x _returnvalue) (.x (Variables|/Game/Blueprints/Camera/LevelsCamera/BP_Room.BP_Room_C|GetfromPos (Variables|Room|GetcurrentRoom))))
              (bind _curve (Timeline|Timeline_2 PlayFromStart)
                (:Update
                  (Transformation|SetWorldLocation _camera (Math|Vector|MakeVector (Math|Float|Lerp (Variables|camera|GetinitXPos) (+ (.x (Variables|/Game/Blueprints/Camera/LevelsCamera/BP_Room.BP_Room_C|GetfromPos (Variables|Room|GetcurrentRoom))) _roomlimits) _curve) (.y _returnvalue_2) (.z _returnvalue_2)) false false)))
              (else
                (bind _curve_2 (Timeline|Timeline_1 PlayFromStart)
                  (:Update
                    (Transformation|SetWorldLocation _camera (Math|Vector|MakeVector (Math|Float|Lerp (Variables|camera|GetinitXPos) (- (.x (Variables|/Game/Blueprints/Camera/LevelsCamera/BP_Room.BP_Room_C|GettoPos (Variables|Room|GetcurrentRoom))) _roomlimits) _curve_2) (.y _returnvalue_2) (.z _returnvalue_2)) false false))))))
          (:then_1
            (Timeline|Timeline_3 PlayFromStart
              (:Finished
                (Variables|Room|SetroomTransition false)))))))
    (:then_1
      (Development|PrintString (Utilities|String|Append "Current Room: " (Utilities|GetDisplayName targetRoom)))
      (Development|PrintString (Utilities|String|Append "Previous Room: " (Utilities|GetDisplayName _output_get))))))

(event EventBeginPlay
  ;[1 1 1] Set this camera as the game camera
  (bind _asbp_character (Utilities|Casting|CastToBP_Character (Game|Player|GetPlayerPawn 0)))
  (Variables|Default|Setplayer _asbp_character)
  (Game|Player|SetViewTargetwithBlend (Game|GetPlayerController 0) self 0.0 "VTBlend_Linear" 0.0 false)
  ;[1 1 1] Set camera init position
  (Transformation|SetWorldLocation (Variables|Default|GetCamera) (Math|Vector|MakeVector (.x (Transformation|GetWorldLocation (Variables|/Script/Engine.Character|GetCapsuleComponent (Variables|Default|Getplayer)))) (.y (Transformation|GetWorldLocation (Variables|Default|GetCamera))) (+ (.z (Transformation|GetWorldLocation (Variables|/Script/Engine.Character|GetCapsuleComponent (Variables|Default|Getplayer)))) (Variables|camera|GetcamVerticalOffset))) false false))

(event EventTick
  (params (DeltaSeconds :type Float%20%28single-precision%29))
  (bind _camera (Variables|Default|GetCamera))
  (bind _currentroom (Variables|Room|GetcurrentRoom))
  (bind _roomlimits (Variables|Room|GetroomLimits))
  (bind _camera_2 (Variables|Default|GetCamera))
  (bind _returnvalue (Transformation|GetWorldLocation _camera))
  (bind _returnvalue_2 (Transformation|GetWorldLocation _camera_2))
  ;[1 1 1] Camera x y pos
  (if (not (Variables|Room|GetroomTransition))
    ;;[1 1 1] Normal conditions
    (Transformation|SetWorldLocation (Variables|Default|GetCamera) (Math|Vector|MakeVector (Math|Float|Clamp(Float) (.x (Transformation|GetWorldLocation (Variables|/Script/Engine.Character|GetCapsuleComponent (Variables|Default|Getplayer)))) (- (.x (Variables|/Game/Blueprints/Camera/LevelsCamera/BP_Room.BP_Room_C|GettoPos _currentroom)) _roomlimits) (+ (.x (Variables|/Game/Blueprints/Camera/LevelsCamera/BP_Room.BP_Room_C|GetfromPos _currentroom)) _roomlimits)) (.y _returnvalue_2) (.z _returnvalue_2)) false false)
    (Utilities|FlowControl|Sequence
      (:then_0
        ;[1 1 1] Camera z pos
        (bind (_outofbox _playerabovecamera) (CallFunction|IsPlayerOutsideBox))
        (if _outofbox
          (Utilities|FlowControl|Sequence
            (:then_0
              (bind _camplayerdiff (CallFunction|CamPlayerZDiff _playerabovecamera))
              (Transformation|SetWorldLocation _camera (Math|Vector|MakeVector (.x _returnvalue) (.y _returnvalue) _camplayerdiff) false false)))))
      (:then_1))))

(fn ConstructionScript
  (Variables|general|SetfromPos (Transformation|GetWorldLocation (Variables|Default|GetfromSphere)))
  (Variables|general|SettoPos (Transformation|GetWorldLocation (Variables|Default|GettoSphere)))
  (Transformation|SetRelativeLocation (Variables|Default|GetCamera) (Math|Vector|MakeVector 0.0 (Variables|camera|Getdistance) 0.0) false false)
  (Transformation|SetRelativeRotation (Variables|Default|GetCamera) (Math|Rotator|MakeRotator 0.0 (Variables|camera|Getpitch) 9e+01) false false)
  (Variables|Room|SetcurrentRoom (Utilities|Array|Get(acopy) (Variables|Room|Getrooms))))

(fn IsPlayerOutsideBox
  (bind _boundingbox (Variables|BoundingBox|GetboundingBox))
  (bind _camverticaloffset (Variables|camera|GetcamVerticalOffset))
  (bind _camera (Variables|Default|GetCamera))
  (bind _bbverticaloffset (Variables|BoundingBox|GetbbVerticalOffset))
  (bind _player (Variables|Default|Getplayer))
  (bind _returnvalue (Transformation|GetWorldLocation _camera))
  (bind _returnvalue_2 (+ _boundingbox _bbverticaloffset))
  (bind _capsulecomponent (Variables|/Script/Engine.Character|GetCapsuleComponent _player))
  (bind _returnvalue_3 (Transformation|GetWorldLocation _capsulecomponent))
  (bind _returnvalue_4 (- (.z _returnvalue) _camverticaloffset))
  (bind _returnvalue_5 (+ _returnvalue_4 _returnvalue_2))
  (bind _returnvalue_6 (>= (.z _returnvalue_3) _returnvalue_5))
  (return (or _returnvalue_6 (<= (.z _returnvalue_3) (- _returnvalue_4 (- _boundingbox _bbverticaloffset)))) _returnvalue_6))

(fn CamPlayerZDiff
  (params (playerAboveCamera :type Boolean))
  (bind _boundingbox (Variables|BoundingBox|GetboundingBox))
  (bind _bbverticaloffset (Variables|BoundingBox|GetbbVerticalOffset))
  (bind _camverticaloffset (Variables|camera|GetcamVerticalOffset))
  (bind _player (Variables|Default|Getplayer))
  (bind _capsulecomponent (Variables|/Script/Engine.Character|GetCapsuleComponent _player))
  (bind _returnvalue (Transformation|GetWorldLocation _capsulecomponent))
  (bind _returnvalue_2 (+ (.z _returnvalue) _camverticaloffset))
  (if playerAboveCamera
    (return (- _returnvalue_2 (+ _boundingbox _bbverticaloffset)))
    (else
      (return (+ _returnvalue_2 (- _boundingbox _bbverticaloffset))))))