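; BP_CameraController is a side-on follow camera that becomes the view target and tracks BP_Character.
; The construction script sets the camera's distance and pitch from variables and stores two sphere marker positions, which go unused here.
; BeginPlay applies a vertical offset, then Tick matches the player's X while keeping Y fixed.
; The BoundingBox height check joins its bounds with OR, so a non-negative value always snaps Z to the player, dropping the offset.
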(event EventBeginPlay
  ;[1 1 1] Set this camera as the game camera
  (bind _asbp_character (Utilities|Casting|CastToBP_Character (Game|Player|GetPlayerPawn 0)))
  (Variables|Default|Setplayer _asbp_character)
  (Game|Player|SetViewTargetwithBlend (Game|GetPlayerController 0) self 0.0 "VTBlend_Linear" 0.0 false)
  ;[1 1 1] Set camera init position
  (Transformation|SetWorldLocation (Variables|Default|GetCamera) (Math|Vector|MakeVector (.x (Transformation|GetWorldLocation (Variables|/Script/Engine.Character|GetCapsuleComponent (Variables|Default|Getplayer)))) (.y (Transformation|GetWorldLocation (Variables|Default|GetCamera))) (+ (.z (Transformation|GetWorldLocation (Variables|/Script/Engine.Character|GetCapsuleComponent (Variables|Default|Getplayer)))) (Variables|camera|GetverticalOffset))) false false))

(event EventTick
  (params (DeltaSeconds :type Float%20%28single-precision%29))
  (bind _camera (Variables|Default|GetCamera))
  (bind _camera_2 (Variables|Default|GetCamera))
  (bind _camera_3 (Variables|Default|GetCamera))
  (bind _player (Variables|Default|Getplayer))
  (bind _boundingbox (Variables|BoundingBox|GetboundingBox))
  (bind _returnvalue (Transformation|GetWorldLocation _camera_3))
  (bind _returnvalue_2 (Transformation|GetWorldLocation _camera))
  (bind _returnvalue_3 (Transformation|GetWorldLocation _camera_2))
  (bind _capsulecomponent (Variables|/Script/Engine.Character|GetCapsuleComponent _player))
  (bind _returnvalue_4 (Transformation|GetWorldLocation _capsulecomponent))
  ;[1 1 1] Camera x y pos
  (Transformation|SetWorldLocation (Variables|Default|GetCamera) (Math|Vector|MakeVector (.x (Transformation|GetWorldLocation (Variables|/Script/Engine.Character|GetCapsuleComponent (Variables|Default|Getplayer)))) (.y _returnvalue_2) (.z _returnvalue_2)) false false)
  ;[1 1 1] Camera z pos
  (if (or (<= (.z _returnvalue) (+ (.z _returnvalue_4) _boundingbox)) (>= (.z _returnvalue) (- (.z _returnvalue_4) _boundingbox)))
    (Transformation|SetWorldLocation (Variables|Default|GetCamera) (Math|Vector|MakeVector (.x _returnvalue_3) (.y _returnvalue_3) (.z (Transformation|GetWorldLocation (Variables|/Script/Engine.Character|GetCapsuleComponent (Variables|Default|Getplayer))))) false false)))

(fn ConstructionScript
  (Variables|general|SetfromPos (Transformation|GetWorldLocation (Variables|Default|GetfromSphere)))
  (Variables|general|SettoPos (Transformation|GetWorldLocation (Variables|Default|GettoSphere)))
  (Transformation|SetRelativeLocation (Variables|Default|GetCamera) (Math|Vector|MakeVector 0.0 (Variables|camera|Getdistance) 0.0) false false)
  (Transformation|SetRelativeRotation (Variables|Default|GetCamera) (Math|Rotator|MakeRotator 0.0 (Variables|camera|Getpitch) 9e+01) false false))