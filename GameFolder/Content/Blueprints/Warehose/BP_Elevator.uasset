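; Elevator trigger actor that lets the player raise a referenced actor, MeshMove, with the E key.
; BP_Character overlapping the Box toggles the Indication and enables or disables input, guarded by the TriggerOn flag.
; Pressing E instantly offsets MeshMove upward without sweep, then destroys this actor, making it single-use.
; An effect spawn on Button and a debug print follow the destroy call.
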(event OnComponentBeginOverlap(Box)
  (params (OverlappedComponent :type Primitive%20Component%20Object%20Reference) (OtherActor :type Actor%20Object%20Reference) (OtherComp :type Primitive%20Component%20Object%20Reference) (OtherBodyIndex :type Integer) (bFromSweep :type Boolean) (SweepResult :type Hit%20Result%20Structure%20%28by%20ref%29))
  (Utilities|Casting|CastToBP_Character OtherActor)
  (bind _output_get (Variables|Default|SettriggerOn (Variables|Default|GettriggerOn)))
  (if _output_get
    (Rendering|ToggleVisibility (Variables|Default|GetIndication) false)
    (Variables|Default|SettriggerOn false)
    (Input|EnableInput (Game|GetPlayerController 0))))

(event OnComponentEndOverlap(Box)
  (params (OverlappedComponent :type Primitive%20Component%20Object%20Reference) (OtherActor :type Actor%20Object%20Reference) (OtherComp :type Primitive%20Component%20Object%20Reference) (OtherBodyIndex :type Integer))
  (Utilities|Casting|CastToBP_Character OtherActor)
  (if (not (Variables|Default|GettriggerOn))
    (Rendering|ToggleVisibility (Variables|Default|GetIndication) false)
    (Variables|Default|SettriggerOn true)
    (Input|DisableInput (Game|GetPlayerController 0))))

(event EventBeginPlay)

(event Collision|EventActorBeginOverlap
  (params (OtherActor :type Actor%20Object%20Reference)))

(event EventTick
  (params (DeltaSeconds :type Float%20%28single-precision%29)))

(event Input|KeyboardEvents|E
  (params (Key :type Key%20Structure :default "None"))
  (:Pressed
    (Transformation|AddActorWorldOffset (Variables|Default|GetMeshMove) "0, 0,700.000000")
    (Actor|DestroyActor)
    (Niagara|SpawnSystemAttached (Variables|Default|GetNewVar_0) (Variables|Default|GetButton) "None" "0, 0, 0" "0, 0, 0" "KeepRelativeOffset" false)
    (Development|PrintString "Hello")))

(fn ConstructionScript
  (Variables|Default|SetMeshMove (Variables|Default|GetMeshMove)))