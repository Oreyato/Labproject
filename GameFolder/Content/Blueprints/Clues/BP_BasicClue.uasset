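; BP_BasicClue is a collectible clue pickup that unlocks its entry when a Player-tagged actor overlaps it.
; Construction looks up the DT_Clues row named by ClueIndex to fill its clue data, and BeginPlay attaches a Niagara effect to the cube.
; Overlap sets IsUnlocked in GI_Clues' Clues array, calls DestroyActor, then spawns a collect explosion on the cube.
; Button prompt and input condition are unwired placeholder prints, so pickup is immediate.
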(event EventBeginPlay
  (Niagara|SpawnSystemAttached (Variables|Default|GetNiagaraRef) (Variables|Default|GetCube) "None" "0, 0, 0" "0, 0, 0" "KeepRelativeOffset" true))

(event Collision|EventActorBeginOverlap
  (params (OtherActor :type Actor%20Object%20Reference))
  (bind _returnvalue (Game|GetGameInstance))
  (bind _clueindex (Variables|Default|GetclueIndex))
  (bind _asgi_clues (Utilities|Casting|CastToGI_Clues _returnvalue))
  (bind _clues (Variables|/Game/Blueprints/GI_Clues.GI_Clues_C|Getclues _asgi_clues))
  (bind _output (Utilities|Array|Get(acopy) _clues _clueindex))
  (if (Actor|ActorHasTag OtherActor "Player")
    (Development|PrintString "In")
    (if true
      (Development|PrintString (Utilities|String|ToString(Boolean) (.isUnlocked (Utilities|Struct|BreakStruct_Clue _output))))
      (bind _structout (Utilities|Struct|SetmembersinStruct_Clue _output true))
      (Development|PrintString (Utilities|String|ToString(Boolean) (.isUnlocked (Utilities|Struct|BreakStruct_Clue _structout))))
      (Actor|DestroyActor)
      (Niagara|SpawnSystemAttached "/Game/Niagara_Système/NA_ObjectCollect_Explosion.NA_ObjectCollect_Explosion" (Variables|Default|GetCube) "None" "0, 0, 0" "0, 0, 0" "KeepRelativeOffset" true))))

(event Collision|EventActorEndOverlap
  (params (OtherActor :type Actor%20Object%20Reference))
  (if (Actor|ActorHasTag OtherActor "Player")
    (Development|PrintString "Out")))

(fn ConstructionScript
  (bind _returnvalue (Utilities|GetDataTableRow "/Game/Blueprints/EvidenceBoard/DT_Clues.DT_Clues" (Utilities|String|StringToName (Utilities|String|ToString(Integer) (Variables|Default|GetclueIndex))))
    (:then
      (bind _output_get (Variables|Default|Setclue _returnvalue))
      (Variables|Default|SetclueName (.name (Utilities|Struct|BreakStruct_Clue _output_get)))
      (Variables|Default|SetNiagaraRef (Variables|Default|GetNiagaraRef)))))